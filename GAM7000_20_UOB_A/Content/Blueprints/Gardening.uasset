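; Gardening interaction actor that lets the player start a gardening minigame and earn happiness for completing it.
; Overlapping its Box enables input outside race levels and leaving disables it, while F opens the GardeningMiniGame widget.
; The CompletedGardening event adds one happiness to Player1 and destroys the Box so the spot stops triggering.
; A separate GrabbingTrowel function flags the trowel as selected.
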(event `self.ReceiveBeginPlay`
  (bind _asplayer_1 (cast `/Game/Blueprints/Player1` (`GameplayStatics.GetPlayerCharacter` 0)))
  (set `self.PlayerReference` _asplayer_1))

(event `self.Box.OnComponentBeginOverlap`
  (params (OverlappedComponent :type "PrimitiveComponent Object Reference") (OtherActor :type "Actor Object Reference") (OtherComp :type "PrimitiveComponent Object Reference") (OtherBodyIndex :type Integer) (bFromSweep :type Boolean) (SweepResult :type "HitResult Structure (by ref)"))
  ;[1 1 1] Enable/Disable Player Input
  (if (not (`/Game/Blueprints/Player1.isRaceLevel` (`self.PlayerReference`)))
    (`self.EnableInput` (`.ReturnValue` (`VictoryBPFunctionLibrary.Accessor__GetPlayerController` (`GameplayStatics.GetPlayerCharacter` 0))))))

(event `self.Box.OnComponentEndOverlap`
  (params (OverlappedComponent :type "PrimitiveComponent Object Reference") (OtherActor :type "Actor Object Reference") (OtherComp :type "PrimitiveComponent Object Reference") (OtherBodyIndex :type Integer))
  ;[1 1 1] Enable/Disable Player Input
  (`self.DisableInput` (`.ReturnValue` (`VictoryBPFunctionLibrary.Accessor__GetPlayerController` (`GameplayStatics.GetPlayerCharacter` 0)))))

(event `Key|F`
  (params (Key :type "Key Structure"))
  (:`Pressed`
    (if (not (`/Game/Blueprints/Player1.isRaceLevel` (`self.PlayerReference`)))
      (bind _returnvalue (`|CreateWidget` "/Game/Blueprints/GardeningUI/GardeningMiniGame.GardeningMiniGame_C" (`.ReturnValue` (`VictoryBPFunctionLibrary.Accessor__GetPlayerController` (`GameplayStatics.GetPlayerCharacter` 0)))))
      (bind _output_get (set `self.GardeningMiniGame` _returnvalue))
      (`UserWidget.AddToViewport` _output_get 0))))

(event `CompletedGardening`
  ;[1 1 1] Completing Task
  (`KismetSystemLibrary.PrintString` "Task Completed")
  ;[1 1 1] Adding To Happiness
  (bind _asplayer_1 (cast `/Game/Blueprints/Player1` (`GameplayStatics.GetPlayerCharacter` 0))
    (:`then`
      (`/Game/Blueprints/Player1.Plus1ToHappiness` _asplayer_1)
      (`ActorComponent.K2_DestroyComponent` (`self.Box`)))
    (:`CastFailed`
      (`KismetSystemLibrary.PrintString` "Not Working"))))

(fn `GrabbingTrowel`
  (if (`self.TrowelSelected?`)
    (`KismetSystemLibrary.PrintString` "Trowel Grabbed already")
    (else
      (set `self.TrowelSelected?` true))))

(fn `UserConstructionScript`)