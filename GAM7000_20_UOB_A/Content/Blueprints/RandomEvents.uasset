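; RandomEvents is a trigger actor that starts a random event for the player on overlap.
; It caches the Player1 character on BeginPlay.
; Any actor overlap shows an event widget for one second, then removes it, destroys the Box component and sets the player's RandomEvent flag to true.
; The overlapping actor is not checked, and the event itself is not handled here.
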(event `self.ReceiveBeginPlay`
  (bind _asplayer_1 (cast `/Game/Blueprints/Player1` (`GameplayStatics.GetPlayerCharacter` 0)))
  (set `self.PlayerRef` _asplayer_1))

(event `self.ReceiveActorBeginOverlap`
  (params (OtherActor :type "Actor Object Reference"))
  (bind _returnvalue (`|CreateWidget` "/Game/Blueprints/EventUI.EventUI_C" (`.ReturnValue` (`VictoryBPFunctionLibrary.Accessor__GetPlayerController` (`GameplayStatics.GetPlayerCharacter` 0)))))
  (`UserWidget.AddToViewport` _returnvalue 0)
  (`KismetSystemLibrary.Delay` 1.0)
  (`Widget.RemoveFromParent` _returnvalue)
  (`ActorComponent.K2_DestroyComponent` (`self.Box`))
  (set `/Game/Blueprints/Player1.RandomEvent?` true (`self.PlayerRef`)))

(fn `UserConstructionScript`)